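; BP_Enemy is an enemy actor in InfiniteMatrix that damages the player on contact and can be shot for points.
; It sets a short life span at BeginPlay, so unhandled enemies clean themselves up.
; Overlapping BP_Player decrements Health, destroys the enemy, updates IsDead and shows the restart display on death.
; Overlapping BP_Bullet destroys both actors and adds to the player's Score.
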(event `self.ReceiveBeginPlay`
  (`self.SetLifeSpan` 8.0))

(event `self.ReceiveActorBeginOverlap`
  (params (OtherActor :type "Actor Object Reference"))
  (bind _asbp_player (cast `/Game/InfiniteMatrix/Blueprints/BP_Player` OtherActor)
    (:`then`
      (bind _result (`/Engine/EditorBlueprintResources/StandardMacros.DecrementInt` (`/Game/InfiniteMatrix/Blueprints/BP_Player.Health` _asbp_player))
        (:`  `
          (`self.K2_DestroyActor`)
          (bind _output_get (set `/Game/InfiniteMatrix/Blueprints/BP_Player.IsDead` (< _result 1) _asbp_player))
          (if _output_get
            (`/Game/InfiniteMatrix/Blueprints/BP_Player.DisplayRestart` _asbp_player)))))
    (:`CastFailed`
      (bind _asbp_bullet (cast `/Game/InfiniteMatrix/Blueprints/BP_Bullet` OtherActor))
      (`self.K2_DestroyActor` _asbp_bullet)
      (`self.K2_DestroyActor`)
      (bind _asbp_player_2 (cast `/Game/InfiniteMatrix/Blueprints/BP_Player` (`GameplayStatics.GetPlayerPawn` 0)))
      (set `/Game/InfiniteMatrix/Blueprints/BP_Player.Score` (+ (`/Game/InfiniteMatrix/Blueprints/BP_Player.Score` _asbp_player_2) 25) _asbp_player_2))))

(fn `UserConstructionScript`)